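; An interactable unlock trigger that lets the player unlock a referenced door by pressing E while overlapping it.
; Overlap begin and end with the player pawn enable and disable input on the actor, with an on-screen prompt on entry.
; Pressing E sets the target door's IsLocked to false and prints a confirmation message.
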(event `self.ReceiveActorBeginOverlap`
  (params (OtherActor :type "Actor Object Reference"))
  (if (== OtherActor (`GameplayStatics.GetPlayerPawn` 0))
    (`self.EnableInput` (`GameplayStatics.GetPlayerController` 0))
    (`KismetSystemLibrary.PrintString` "Press E key to unlock the door")))

(event `self.ReceiveActorEndOverlap`
  (params (OtherActor :type "Actor Object Reference"))
  (if (== OtherActor (`GameplayStatics.GetPlayerPawn` 0))
    (`self.DisableInput` (`GameplayStatics.GetPlayerController` 0))))

(event `Key|E`
  (params (Key :type "Key Structure"))
  ;[1 1 1] When the E key is pressed, unlock the door
  (:`Pressed`
    (set `/Game/Blueprints/BP_LockedDoor.isLocked` false (`self.DoorToUnlock`))
    (`KismetSystemLibrary.PrintString` "The door was unlocked")))

(fn `UserConstructionScript`)
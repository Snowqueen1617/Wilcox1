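; BP_CreepyLight is an overlap trigger that lights up a referenced Light actor and starts a level sequence for a creepy lighting effect.
; The light starts at zero intensity on BeginPlay and brightens when the player pawn begins overlapping.
; When any actor stops overlapping, the referenced sequence plays on an endless loop.
; Nothing in the Blueprint dims the light or stops the sequence afterwards.
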(event `self.ReceiveBeginPlay`
  (`LightComponent.SetIntensity` (`Light.LightComponent` (`self.Light`)) 0.0))

(event `self.ReceiveActorBeginOverlap`
  (params (OtherActor :type "Actor Object Reference"))
  (if (== (`GameplayStatics.GetPlayerPawn` 0) null)
    (`LightComponent.SetIntensity` (`Light.LightComponent` (`self.Light`)) 135.0)))

(event `self.ReceiveActorEndOverlap`
  (params (OtherActor :type "Actor Object Reference"))
  (`MovieSceneSequencePlayer.PlayLooping` (`LevelSequenceActor.SequencePlayer` (`self.Sequence`)) -1))

(fn `UserConstructionScript`)
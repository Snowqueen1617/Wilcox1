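; BP_LockedDoor is a door that reacts when the player pawn overlaps it, based on its IsLocked flag.
; If locked, it writes LockedDoorText to a referenced text renderer; otherwise it plays the OpenDoorSequence level sequence.
; The flag is only read here, and there is no end-overlap handling to clear the text or close the door.
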(event `self.ReceiveActorBeginOverlap`
  (params (OtherActor :type "Actor Object Reference"))
  (if (== OtherActor (`GameplayStatics.GetPlayerPawn` 0))
    (if (`self.isLocked`)
      (`TextRenderComponent.K2_SetText` (`TextRenderActor.TextRender` (`self.lockedDoorTextRenderer`)) (`KismetTextLibrary.Conv_StringToText` (`self.lockedDoorText`)))
      (else
        (`MovieSceneSequencePlayer.Play` (`LevelSequenceActor.SequencePlayer` (`self.OpenDoorSequence`)))))))

(fn `UserConstructionScript`)
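; Trigger box that acts as a password prompt to unlock a linked sliding glass door.
; When the player pawn overlaps it, it enables input and prints a password question, then disables input when the pawn leaves.
; While input is enabled, pressing Q, the hardcoded answer, clears the referenced door's IsLocked flag and prints an unlock message.
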(event `self.ReceiveActorBeginOverlap`
  (params (OtherActor :type "Actor Object Reference"))
  (if (== OtherActor (`GameplayStatics.GetPlayerPawn` 0))
    (`self.EnableInput` (`GameplayStatics.GetPlayerController` 0))
    ;[1 1 1] The answer is Q
    (`KismetSystemLibrary.PrintString` "What is the password?")))

(event `self.ReceiveActorEndOverlap`
  (params (OtherActor :type "Actor Object Reference"))
  (if (== OtherActor (`GameplayStatics.GetPlayerPawn` 0))
    (`self.DisableInput` (`GameplayStatics.GetPlayerController` 0))))

(event `Key|Q`
  (params (Key :type "Key Structure"))
  ;[1 1 1] When the Q key is pressed, unlock the door
  (:`Pressed`
    (set `/Game/Blueprints/SlidingGlassDoorLocked_Blueprint.isLocked` false (`self.DoorToUnlock`))
    (`KismetSystemLibrary.PrintString` "The door was unlocked")))

(fn `UserConstructionScript`)